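; BP_Wildman is a modular Wildman character Blueprint whose look and weapon are assembled from toggleable parts.
; The Construction Script makes the skeletal attachments (horns, eyes, mouths, decor, tail, skull) follow the main Mesh via Set Leader Pose Component.
; It then sets each part's visibility, plus the staff, spear and bat meshes, from per-part boolean variables, so variants are configured without separate Blueprints.
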(fn ConstructionScript
  (Components|SkinnedMesh|SetLeaderPoseComponent (Variables|Default|GetSK_Horn1) (Variables|Character|GetMesh) false false)
  (Utilities|FlowControl|Sequence
    (:then_0
      (Rendering|SetVisibility (Variables|Default|GetSK_Horn1) (Variables|Default|GetHorn1Visability) false))
    (:then_1
      (Rendering|SetVisibility (Variables|Default|GetSK_ArmDecor_2) (Variables|Default|GetArmDecor2Visability) false))
    (:then_2
      (Rendering|SetVisibility (Variables|Default|GetSK_Eye_1) (Variables|Default|GetEye1Visability) false))
    (:then_3
      (Rendering|SetVisibility (Variables|Default|GetSK_Eye_2) (Variables|Default|GetEye2Visability) false))
    (:then_4
      (Rendering|SetVisibility (Variables|Default|GetSK_Eye_3) (Variables|Default|GetEye3Visability) false))
    (:then_5
      (Rendering|SetVisibility (Variables|Default|GetSK_HeadDecor) (Variables|Default|GetHeadDecorVisability) false))
    (:then_6
      (Rendering|SetVisibility (Variables|Default|GetSK_Horn) (Variables|Default|GetHornVisability) false))
    (:then_7
      (Rendering|SetVisibility (Variables|Default|GetSK_ArmDecor_1) (Variables|Default|GetArmDecor1Visability) false))
    (:then_8
      (Rendering|SetVisibility (Variables|Default|GetSK_MaskDecor) (Variables|Default|GetMaskDecorVisability) false))
    (:then_9
      (Rendering|SetVisibility (Variables|Default|GetSK_MaskDecor_Bone) (Variables|Default|GetMaskDecorBoneVisability) false))
    (:then_10
      (Rendering|SetVisibility (Variables|Default|GetSK_Mouth1) (Variables|Default|GetMouth1Visability) false))
    (:then_11
      (Rendering|SetVisibility (Variables|Default|GetSK_Mouth2) (Variables|Default|GetMouth2Visability) false))
    (:then_12
      (Rendering|SetVisibility (Variables|Default|GetSK_Mouth3) (Variables|Default|GetMouth3Visability) false))
    (:then_13
      (Rendering|SetVisibility (Variables|Default|GetSK_Tail) (Variables|Default|GetTailVisability) false))
    (:then_14
      (Rendering|SetVisibility (Variables|Default|GetSK_Scull) (Variables|Default|GetScullVisability) false))
    (:then_15
      (Rendering|SetVisibility (Variables|Default|GetSM_Staff) (Variables|Default|GetStaffVisability) false))
    (:then_16
      (Rendering|SetVisibility (Variables|Default|GetSM_Spear) (Variables|Default|GetSpearVisability) false))
    (:then_17
      (Rendering|SetVisibility (Variables|Default|GetSM_Bat) (Variables|Default|GetBatVisability) false))))
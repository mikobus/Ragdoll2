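; Modular Mimic Book character Blueprint that assembles the creature from a main mesh plus separate tongue and decor skeletal meshes.
; The construction script makes the main mesh the leader pose for both parts, so they follow its animation.
; DecorVisibility and TongueVisibility variables toggle each part at construction.
; It has no runtime logic, as the event graph holds only disabled placeholder events.
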(event EventBeginPlay)

(event Collision|EventActorBeginOverlap
  (params (OtherActor :type Actor%20Object%20Reference)))

(event EventTick
  (params (DeltaSeconds :type Float%20%28single-precision%29)))

(fn ConstructionScript
  (Components|SkinnedMesh|SetLeaderPoseComponent (Variables|Default|GetSKM_MimicBook_Tongue) (Variables|Character|GetMesh) true false)
  (Utilities|FlowControl|Sequence
    (:then_0
      (Rendering|SetVisibility (Variables|Default|GetSKM_MimicBook_Decor) (Variables|Default|GetDecorVisibility) false))
    (:then_1
      (Rendering|SetVisibility (Variables|Default|GetSKM_MimicBook_Tongue) (Variables|Default|GetTongueVisibility) false))))
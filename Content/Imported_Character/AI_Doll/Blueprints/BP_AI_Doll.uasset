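; AI doll character with glowing-eye material on two spheres and a creepy voice line triggered through PlayVoice.
; PlayVoice spawns one sound at a time at half pitch, turns the eyes red, and starts a looping timer.
; The timer eases pitch toward normal while the blackboard's CanMove is true, otherwise slides it down toward zero.
; When the audio finishes, the timer clears and the eyes return to white.
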(event Custom|Play%20Voice
  ;[0 0 0] Voice
  (Variables|Default|GetCurrent%20Audio
    (:then)
    (:else
      (bind _returnvalue (Audio|SpawnSoundatLocation "/Game/Imported_Character/AI_Doll/Sounds/CUE/voice/WAV_I_know_where_you_are_Cue.WAV_I_know_where_you_are_Cue" (Transformation|GetActorLocation) "0, 0, 0" 1.0 0.5 0.0 0 0))
      (bind _output_get (Variables|Default|SetCurrent%20Audio _returnvalue))
      (Rendering|Material|SetVectorParameterValue (Variables|Default|GetDynamic%20Material) "Color" "(R=1.000000,G=0.000000,B=0.000000,A=1.000000)" :!class /Script/Engine.MaterialInstanceDynamic)
      (bind _returnvalue_2 (Utilities|Time|SetTimerbyEvent (delegate Custom|CustomEvent_0) 0.016 true))
      (Variables|Default|SetTimer _returnvalue_2)
      (EventDispatchers|BindEventtoOnAudioFinished _output_get (delegate Custom|CustomEvent_1)))))

(event Custom|CustomEvent_0
  ;[0 0 0] Voice
  (if (ScalableFloat|GetValueasBool (AI|GetBlackboard (Pawn|GetController)) (Utilities|Name|MakeLiteralName "CanMove"))
    (bind _current_audio (Variables|Default|GetCurrent%20Audio)
      (:then
        (Audio|Components|Audio|SetPitchMultiplier _current_audio (Math|Interpolation|FInterpTo (Variables|/Script/Engine.AudioComponent|GetPitchMultiplier (Variables|Default|GetCurrent%20Audio)) 1.0 (Utilities|Time|GetWorldDeltaSeconds) 1.0)))
      (:else))
    (else
      (bind _current_audio_2 (Variables|Default|GetCurrent%20Audio)
        (:then
          (Audio|Components|Audio|SetPitchMultiplier _current_audio_2 (Math|Interpolation|FInterptoConstant (Variables|/Script/Engine.AudioComponent|GetPitchMultiplier (Variables|Default|GetCurrent%20Audio)) 0.0 (Utilities|Time|GetWorldDeltaSeconds) 0.2)))
        (:else)))))

(event Custom|CustomEvent_1
  ;[0 0 0] Voice
  (Utilities|Time|ClearandInvalidateTimerbyHandle (Variables|Default|GetTimer))
  (Rendering|Material|SetVectorParameterValue (Variables|Default|GetDynamic%20Material) "Color" "(R=1.000000,G=1.000000,B=1.000000,A=1.000000)" :!class /Script/Engine.MaterialInstanceDynamic)
  (Variables|Default|SetCurrent%20Audio 0))

(event EventBeginPlay
  ;[0 0 0] Begin Play - Create Dynamic Material
  (bind _returnvalue (Rendering|Material|CreateDynamicMaterialInstance "/Game/Imported_Character/AI_Doll/Demo/Characters/Mannequins/Materials/M_Eye.M_Eye" "None" "None" :!class /Script/Engine.KismetMaterialLibrary))
  (bind _output_get (Variables|Default|SetDynamic%20Material _returnvalue))
  (Rendering|Material|SetMaterial (Variables|Default|GetSphere1) 0 _output_get))

(event EventTick
  (params (DeltaSeconds :type Float%20%28single-precision%29)))

(fn ConstructionScript)
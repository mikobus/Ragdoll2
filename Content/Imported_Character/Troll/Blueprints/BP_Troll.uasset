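; BP_Troll is a modular troll character that layers armor, hair, beard, bottles, decor and a weapon onto a base mesh.
; Its construction script makes the skeletal parts follow the main mesh through Leader Pose and toggles each part and the weapon through visibility variables.
; It also assigns the weapon start and end point references, while BeginPlay only calls the parent implementation.
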(event EventBeginPlay
  (|CallParentFunction))

(event Collision|EventActorBeginOverlap
  (params (OtherActor :type Actor%20Object%20Reference)))

(event EventTick
  (params (DeltaSeconds :type Float%20%28single-precision%29)))

(fn ConstructionScript
  (Variables|Default|SetWeapon%20Endpoint (Variables|Default|GetEnd))
  (Variables|Default|SetWeapon%20Startpoint (Variables|Default|GetStart))
  (Components|SkinnedMesh|SetLeaderPoseComponent (Variables|Default|GetSKM_Decor1) (Variables|Character|GetMesh) true false)
  (Utilities|FlowControl|Sequence
    (:then_0
      (Rendering|SetVisibility (Variables|Default|GetSKM_Decor2) (Variables|Default|GetDecor2_Visibility) false))
    (:then_1
      (Rendering|SetVisibility (Variables|Default|GetSM_Weapon) (Variables|Default|GetWeapon_Visibility) false))
    (:then_3
      (Rendering|SetVisibility (Variables|Default|GetSKM_Armor) (Variables|Default|GetArmor_Visibility) false))
    (:then_4
      (Rendering|SetVisibility (Variables|Default|GetSKM_Hair) (Variables|Default|GetHair_Visibility) false))
    (:then_5
      (Rendering|SetVisibility (Variables|Default|GetSKM_Beard) (Variables|Default|GetBeard_Visibility) false))
    (:then_6
      (Rendering|SetVisibility (Variables|Default|GetSKM_Bottles) (Variables|Default|GetBottles_Visibility) false))
    (:then_7
      (Rendering|SetVisibility (Variables|Default|GetSKM_Decor1) (Variables|Default|GetDecor1_Visibility) false))))
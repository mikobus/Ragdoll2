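; Actor that drives a player-following attract/repulse field for dynamic bug Niagara effects through the NPC_DynamicBugsNiagaraCollection parameter collection.
; BeginPlay sets a negative force strength, and Tick writes the player pawn's location and a speed-based radius into the collection.
; The radius interpolates at constant rate, growing quickly as the player speeds up and shrinking slowly afterward.
; A Sphere component follows the player to visualize that radius.
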(event EventTick
  (params (DeltaSeconds :type Float%20%28single-precision%29))
  (bind _returnvalue (Game|Player|GetPlayerPawn 0))
  (bind _returnvalue_2 (Game|Player|GetPlayerPawn 0))
  (bind _sphere (Variables|Default|GetSphere))
  (bind _returnvalue_3 (Transformation|GetActorLocation _returnvalue_2))
  (bind _returnvalue_4 (Transformation|GetVelocity _returnvalue))
  (bind _returnvalue_5 (Math|Vector|VectorLength _returnvalue_4))
  (bind _returnvalue_6 (Math|Float|MapRangeClamped _returnvalue_5 0.0 3e+02 0.0 222.0))
  (bind _returnvalue_7 (Class|NiagaraFunctionLibrary|GetNiagaraParameterCollection "/Game/Imported_Character/DynamicBugs/NiagaraSystem/NPC_DynamicBugsNiagaraCollection.NPC_DynamicBugsNiagaraCollection"))
  (bind _returnvalue_8 (Class|NiagaraParameterCollectionInstance|GetFloatParameter _returnvalue_7 "NewNiagaraFloat"))
  ;[1 1 1] Repulse/Attract radius
  (Effects|Components|ParticleSystem|SetFloatParameter _returnvalue_7 "NewNiagaraFloat" (Math|Interpolation|FInterptoConstant _returnvalue_8 _returnvalue_6 (Utilities|Time|GetWorldDeltaSeconds) (Math|Float|SelectFloat 5e+01 1e+03 (> _returnvalue_8 _returnvalue_6))))
  ;[1 1 1] Repulse/Attract world location
  (Effects|Components|ParticleSystem|SetVectorParameter _returnvalue_7 "NewVector3f" _returnvalue_3)
  ;[1 1 1] Visualize attract/repulse Radius
  (Components|Sphere|SetSphereRadius _sphere (Math|Interpolation|FInterptoConstant _returnvalue_8 _returnvalue_6 (Utilities|Time|GetWorldDeltaSeconds) (Math|Float|SelectFloat 5e+01 1e+03 (> _returnvalue_8 _returnvalue_6))) true)
  (Transformation|SetWorldLocation _sphere _returnvalue_3 false false))

(event EventBeginPlay
  (bind _returnvalue (Class|NiagaraFunctionLibrary|GetNiagaraParameterCollection "/Game/Imported_Character/DynamicBugs/NiagaraSystem/NPC_DynamicBugsNiagaraCollection.NPC_DynamicBugsNiagaraCollection"))
  ;[1 1 1] Change attract/repulse strength
  (Effects|Components|ParticleSystem|SetFloatParameter _returnvalue "NiagaraFloat" -5e+02))

(fn ConstructionScript)